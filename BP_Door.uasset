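; Door actor that swings open and closed, either automatically as a character enters and leaves its trigger or by pressing E inside it.
; A gate enables the key only during overlap in manual mode, and a DoorOpen flag toggles the state.
; SwingOpen and SwingClosed timelines lerp the door's relative rotation.
; When Is2Sided is set, the character's position in door space picks the yaw direction, so it opens away from them.
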(event OnComponentBeginOverlap(Trigger)
  (params (OverlappedComponent :type Primitive%20Component%20Object%20Reference) (OtherActor :type Actor%20Object%20Reference) (OtherComp :type Primitive%20Component%20Object%20Reference) (OtherBodyIndex :type Integer) (bFromSweep :type Boolean) (SweepResult :type Hit%20Result%20Structure%20%28by%20ref%29))
  (bind _door (Variables|Default|GetDoor))
  (bind _door_2 (Variables|Default|GetDoor))
  (if (Variables|Default|GetIsAuto)
    (bind _asthird_person_character (Utilities|Casting|CastToThirdPersonCharacter OtherActor))
    (Variables|Default|SetLocation (Transformation|GetActorLocation _asthird_person_character))
    (Audio|Components|Audio|Stop (Variables|Default|GetSwing%20closed))
    (if (Variables|Default|GetIs2Sided)
      (Variables|Default|SetOpen%20direction (> (.X (Math|Vector|BreakVector (Math|Vector|UnrotateVector (- (Transformation|GetActorLocation) (Variables|Default|GetLocation)) (Transformation|GetActorRotation)))) 0.0))
      (bind _rotation (Timeline|Swing%20open PlayFromStart)
        (:Update
          (Transformation|SetRelativeRotation _door_2 (Math|Rotator|Lerp(Rotator) (Variables|/Script/Engine.SceneComponent|GetRelativeRotation _door_2) (Math|Rotator|MakeRotator 0.0 0.0 (Math|Float|SelectFloat -9e+01 9e+01 (Variables|Default|GetOpen%20direction))) _rotation true) false false)))
      (else
        (Timeline|Swing%20open PlayFromStart)))
    (else
      (Utilities|FlowControl|Gate true) ; enters at Open
    )))

(event OnComponentEndOverlap(Trigger)
  (params (OverlappedComponent :type Primitive%20Component%20Object%20Reference) (OtherActor :type Actor%20Object%20Reference) (OtherComp :type Primitive%20Component%20Object%20Reference) (OtherBodyIndex :type Integer))
  (bind _door (Variables|Default|GetDoor))
  (bind _door_2 (Variables|Default|GetDoor))
  (if (Variables|Default|GetIsAuto)
    (Audio|Components|Audio|Stop (Variables|Default|GetSwing%20open))
    (bind _rotation (Timeline|Swing%20closed PlayFromStart)
      (:Update
        (Transformation|SetRelativeRotation _door (Math|Rotator|Lerp(Rotator) (Variables|/Script/Engine.SceneComponent|GetRelativeRotation _door) "0, 0, 0" _rotation true) false false)))
    (else
      (Utilities|FlowControl|Gate true) ; enters at Close
    )))

(event Input|KeyboardEvents|E
  (params (Key :type Key%20Structure :default "None"))
  (bind _door (Variables|Default|GetDoor))
  (bind _door_2 (Variables|Default|GetDoor))
  (:Pressed
    (Utilities|FlowControl|Gate true
      (:Exit
        (if (Variables|Default|GetDoor%20Open)
          (Variables|Default|SetDoor%20Open false)
          (Audio|Components|Audio|Stop (Variables|Default|GetSwing%20open))
          (bind _rotation (Timeline|Swing%20closed PlayFromStart)
            (:Update
              (Transformation|SetRelativeRotation _door (Math|Rotator|Lerp(Rotator) (Variables|/Script/Engine.SceneComponent|GetRelativeRotation _door) "0, 0, 0" _rotation true) false false)))
          (else
            (Variables|Default|SetDoor%20Open true)
            (bind _asthird_person_character (Utilities|Casting|CastToThirdPersonCharacter (stale OnComponentBeginOverlap(Trigger) OtherActor)))
            (Variables|Default|SetLocation (Transformation|GetActorLocation _asthird_person_character))
            (Audio|Components|Audio|Stop (Variables|Default|GetSwing%20closed))
            (if (Variables|Default|GetIs2Sided)
              (Variables|Default|SetOpen%20direction (> (.X (Math|Vector|BreakVector (Math|Vector|UnrotateVector (- (Transformation|GetActorLocation) (Variables|Default|GetLocation)) (Transformation|GetActorRotation)))) 0.0))
              (bind _rotation_2 (Timeline|Swing%20open PlayFromStart)
                (:Update
                  (Transformation|SetRelativeRotation _door_2 (Math|Rotator|Lerp(Rotator) (Variables|/Script/Engine.SceneComponent|GetRelativeRotation _door_2) (Math|Rotator|MakeRotator 0.0 0.0 (Math|Float|SelectFloat -9e+01 9e+01 (Variables|Default|GetOpen%20direction))) _rotation_2 true) false false)))
              (else
                (Timeline|Swing%20open PlayFromStart)))))))))

(fn ConstructionScript)